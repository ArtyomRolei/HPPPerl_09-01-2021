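; SpiderChild_BP is a spider AI pawn Blueprint whose Move event feeds a direction and scale into movement input.
; On BeginPlay it stores the ThirdPersonCharacter as Ron and starts a looping timer on CheckCameraDistance, which is empty.
; Disconnected logic would swap the mesh material when the spider is within a threshold distance of Ron's follow camera, but it never runs.
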(event `self.ReceiveBeginPlay`
  (bind _returnvalue (`GameplayStatics.GetActorOfClass` "/Game/ThirdPersonBP/Blueprints/ThirdPersonCharacter.ThirdPersonCharacter_C"))
  (set `self.Ron` _returnvalue)
  (`KismetSystemLibrary.K2_SetTimerDelegate` (delegate `CheckCameraDistance`) 0.2 true))

(event `Move`
  (params (Direction :type "Vector Structure") (`Scale ` :type "Float (double-precision)"))
  (`self.AddMovementInput` Direction `Scale `))

(event `CheckCameraDistance`)

(fn `UserConstructionScript`)