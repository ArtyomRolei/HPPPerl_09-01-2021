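; Peacock AI character with a fan tail that opens and closes, and which flees when other characters come near.
; At BeginPlay it caches open and closed rotations for each feather scene component, using Scene37 plus random pitch, and staggers animation start.
; Tick eases feathers toward the pose selected by TailOpen/TailClose.
; A looping proximity check triggers audio, closes the tail and briefly runs to a random navigable point at scared speed.
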(event `self.ReceiveBeginPlay`
  (bind (_relativerotation_roll _relativerotation_pitch _relativerotation_yaw) (`KismetMathLibrary.BreakRotator` (`SceneComponent.RelativeRotation` (`self.Scene37`))))
  (`KismetSystemLibrary.K2_SetTimerDelegate` (delegate `rotationChange`) (`KismetMathLibrary.RandomFloatInRange` 5.0 10.0) true)
  (for _array_element (`self.sceneComponentArr`)
    (bind (_relativerotation_roll_2 _relativerotation_pitch_2 _relativerotation_yaw_2) (`KismetMathLibrary.BreakRotator` (`SceneComponent.RelativeRotation` _array_element)))
    (`KismetArrayLibrary.Array_Add` (`self.sceneStruct`) (make `/Game/AI/Peacock/PeacockFeatherStruct` _array_element (`KismetMathLibrary.MakeRotator` _relativerotation_roll_2 _relativerotation_pitch_2 _relativerotation_yaw_2) (`KismetMathLibrary.MakeRotator` _relativerotation_roll (+ _relativerotation_pitch (`KismetMathLibrary.RandomFloatInRange` -20.0 20.0)) _relativerotation_yaw))))
  (for _array_element_2 (`self.sceneStruct`)
    (`SceneComponent.K2_SetRelativeRotation` (break `/Game/AI/Peacock/PeacockFeatherStruct` _array_element_2) (`.RotationWhenTailClose_7_B58D61F642E2490DBCFA088D7AAF24A7` (break `/Game/AI/Peacock/PeacockFeatherStruct` _array_element_2)) false false)
    (set `SkeletalMeshComponent.bPauseAnims` true (`self.Mesh`))
    (`|ExecutionSequence`
      (:`then_0`
        (`KismetSystemLibrary.K2_SetTimerDelegate` (delegate `ListenHumans`) 1.0 true))
      (:`then_1`
        (`KismetSystemLibrary.Delay` (`KismetMathLibrary.RandomFloatInRange` 0.0 10.0))
        (set `SkeletalMeshComponent.bPauseAnims` false (`self.Mesh`))))))

(event `ListenHumans`
  (bind _audio (`self.Audio`))
  (bind _outactors (`GameplayStatics.GetAllActorsOfClass` "/Script/Engine.Character"))
  (for _array_element _outactors
    (cast `/Game/AI/Peacock/PeacockChar_BP` _array_element
      (:`CastFailed`
        (if (<= (`KismetMathLibrary.Vector_Distance` (`self.K2_GetActorLocation`) (`self.K2_GetActorLocation` _array_element)) (`self.DistanceForScare`))
          (if (not (`self.scarred`))
            (set `self.scarred` true)
            (if (not (`AudioComponent.IsPlaying` _audio))
              (`AudioComponent.Play` _audio 0.0))
            (`self.TailClose`)
            (`self.Start Moving` 1500.0)
            (set `CharacterMovementComponent.MaxWalkSpeed` (`self.walkSpeedScarry`) (`self.CharacterMovement`))
            (`KismetSystemLibrary.Delay` 3.0)
            (`Controller.StopMovement` (`AIBlueprintHelperLibrary.GetAIController` self))
            (set `self.scarred` false)
            (set `CharacterMovementComponent.MaxWalkSpeed` (`self.walkSpeedCalm`) (`self.CharacterMovement`))))))))

(event `rotationChange`)

(event `Start Moving`
  (params (DistanceForRandomMoving :type "Float (double-precision)" :default 500.0))
  (`AIController.MoveToLocation` (`AIBlueprintHelperLibrary.GetAIController` self) (`NavigationSystemV1.K2_GetRandomLocationInNavigableRadius` (`self.K2_GetActorLocation`) DistanceForRandomMoving null null) 20.0 false true false true null true))

(event `End Moving`
  (if (not (`self.scarred`))
    (`Controller.StopMovement` (`AIBlueprintHelperLibrary.GetAIController` self))))

(event `TailOpen`
  (set `self.OpenTail` true))

(event `TailClose`
  (set `self.OpenTail` false))

(event `self.ReceiveTick`
  (params (DeltaSeconds :type "Float (single-precision)"))
  (bind _rinterpspeed (`self.RinterpSpeed`))
  (if (`self.OpenTail`)
    (for _array_element (`self.sceneStruct`)
      (`SceneComponent.K2_SetRelativeRotation` (break `/Game/AI/Peacock/PeacockFeatherStruct` _array_element) (`|EaseFunction` "Linear" _rinterpspeed (`SceneComponent.RelativeRotation` (break `/Game/AI/Peacock/PeacockFeatherStruct` _array_element)) (`.RotationWhenTailOpen_5_35ABA7624F4CC1028E5F0CA672BBE4F9` (break `/Game/AI/Peacock/PeacockFeatherStruct` _array_element))) false false))
    (else
      (for _array_element_2 (`self.sceneStruct`)
        (`SceneComponent.K2_SetRelativeRotation` (break `/Game/AI/Peacock/PeacockFeatherStruct` _array_element_2) (`|EaseFunction` "Linear" _rinterpspeed (`SceneComponent.RelativeRotation` (break `/Game/AI/Peacock/PeacockFeatherStruct` _array_element_2)) (`.RotationWhenTailClose_7_B58D61F642E2490DBCFA088D7AAF24A7` (break `/Game/AI/Peacock/PeacockFeatherStruct` _array_element_2))) false false)))))

(fn `UserConstructionScript`
  (set `self.sceneComponentArr` (`|MakeArray` (`self.Scene19`) (`self.Scene2`) (`self.Scene3`) (`self.Scene4`) (`self.Scene5`) (`self.Scene6`) (`self.Scene7`) (`self.Scene8`) (`self.Scene9`) (`self.Scene10`) (`self.Scene11`) (`self.Scene12`) (`self.Scene13`) (`self.Scene14`) (`self.Scene15`) (`self.Scene16`) (`self.Scene17`) (`self.Scene18`) (`self.Scene1`) (`self.Scene20`) (`self.Scene21`) (`self.Scene22`) (`self.Scene23`) (`self.Scene24`) (`self.Scene25`) (`self.Scene26`) (`self.Scene27`) (`self.Scene28`) (`self.Scene29`) (`self.Scene30`) (`self.Scene31`) (`self.Scene32`) (`self.Scene33`) (`self.Scene34`) (`self.Scene35`) (`self.Scene36`))))