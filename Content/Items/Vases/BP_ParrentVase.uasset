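; BP_ParentVase is a base breakable vase with an empty PostAnyDamage hook for child-specific behavior.
; AnyDamage plays a break sound every time, while the first hit calls the hook and may drop a chicken leg.
; Damage applies radial damage and a destructible impulse from Ron's capsule, throttled by a timer-reset DoOnce.
; The resurection event spawns VaseResurrection, waits, then replaces the actor with a fresh instance of its own class.
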(event `self.ReceiveAnyDamage`
  (params (Damage :type "Float (single-precision)") (DamageType :type "DamageType Object Reference") (InstigatedBy :type "Controller Object Reference") (DamageCauser :type "Actor Object Reference"))
  (`GameplayStatics.PlaySoundAtLocation` "/Game/Sounds/Vases/VaseDestroed_Cue.VaseDestroed_Cue" (`self.K2_GetActorLocation`) (struct) 1.0 1.0 0.0 null null null)
  (if (not (`self.isDamaged`))
    (set `self.isDamaged` true)
    (`self.postAnyDamage`)
    (if (`KismetMathLibrary.RandomBoolWithWeight` 0.3)
      (`|SpawnActorFromClass` "/Game/Items/Eat/ChickenLeg/ChickenLegBP.ChickenLegBP_C" (`self.GetTransform`) "AlwaysSpawn" "OverrideRootScale" null null))))

(event `resurection`
  (`|SpawnActorFromClass` "/Game/FX/Magic/VaseResurrection/VaseResurrection.VaseResurrection_C" (`self.GetTransform`) "AlwaysSpawn" "OverrideRootScale" null null)
  (`KismetSystemLibrary.Delay` (`self.timerForResurection`))
  (`|SpawnActorFromClass` (`GameplayStatics.GetObjectClass` self) (`self.GetTransform`) "AlwaysSpawn" "OverrideRootScale" null null)
  (`self.K2_DestroyActor`))

(event `Damage`
  (params (Capsule :type "SceneComponent Object Reference") (Ron :type "/Game/ThirdPersonBP/Blueprints/ThirdPersonCharacter Object Reference"))
  (bind _returnvalue (`SceneComponent.K2_GetComponentLocation` Capsule))
  (`/Engine/EditorBlueprintResources/StandardMacros.DoOnce` false :!label _label
    (:`Completed`
      (`GameplayStatics.ApplyRadialDamageWithFalloff` :`BaseDamage` 100.0 :`MinimumDamage` 100.0 :`Origin` _returnvalue :`DamageInnerRadius` 50.0 :`DamageOuterRadius` 50.0 :`DamageFalloff` 1.0 :`DamageCauser` Ron :`InstigatedByController` null :`DamagePreventionChannel` "ECC_WorldDynamic")
      (`PrimitiveComponent.AddImpulse` (`self.Destructible`) (+ _returnvalue (* (`SceneComponent.GetForwardVector` Capsule) 10000.0)) "None" false)
      (`KismetSystemLibrary.K2_SetTimerDelegate` (delegate `resetDoOnceDamage`) 1.0))))

(event `resetDoOnceDamage`
  (goto _label :!via `Reset`))

(fn `postAnyDamage`)

(fn `UserConstructionScript`)